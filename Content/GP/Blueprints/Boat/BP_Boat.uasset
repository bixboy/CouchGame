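; BP_Boat is a boat that animates a repeating, randomized rotation movement from BeginPlay while CanMove is set.
; Each StartMove cycle picks a random ForceStrength and scales the timeline play rate so the cycle lasts a random time between TimeLoopMin and TimeLoopMax.
; The timeline feeds its alpha to UpdateBoatRotation on each update and restarts StartMove on finish, re-rolling strength and duration.
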(event Custom|StartMove
  (if (Variables|Default|GetCanMove)
    (Variables|Default|SetForceStrength (Math|Random|RandomFloatinRange 4.0 1e+01))
    (Components|Timeline|SetPlayRate (Variables|Default|GetTL_BoatMovement) (/ (Components|Timeline|GetTimelineLength (Variables|Default|GetTL_BoatMovement)) (Math|Random|RandomFloatinRange (Variables|Default|GetTimeLoopMin) (Variables|Default|GetTimeLoopMax))))
    (bind _alphamove (Timeline|TL_BoatMovement PlayFromStart)
      (:Update
        (Class|CouchBoat|UpdateBoatRotation _alphamove))
      (:Finished
        (CallFunction|StartMove)))))

(event EventBeginPlay
  (CallFunction|StartMove))

(fn ConstructionScript)