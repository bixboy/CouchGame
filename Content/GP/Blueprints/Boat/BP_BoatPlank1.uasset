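; BP_BoatPlank1 is an interactable boat plank that appears to represent a hole in the boat.
; Shortly after spawning, it plays a 2D explosion sound if its HitMesh world scale marks it as a big hole.
; Overlapping InterractiveBoxRange caches the first BP_CouchCharacter as Player, then initializes the BP_InteractProgress1 widget with this plank.
; Once Player is cached, later overlaps re-initialize the widget without checking the overlapping actor.
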(event OnComponentBeginOverlap(InterractiveBoxRange)
  (params (OverlappedComponent :type Primitive%20Component%20Object%20Reference) (OtherActor :type Actor%20Object%20Reference) (OtherComp :type Primitive%20Component%20Object%20Reference) (OtherBodyIndex :type Integer) (bFromSweep :type Boolean) (SweepResult :type Hit%20Result%20Structure%20%28by%20ref%29))
  (bind _returnvalue (Class|CouchPlank|GetInteractWidget))
  (Variables|Default|GetPlayer
    (:then
      _)
    (:else
      (bind _asbp_couch_character (Utilities|Casting|CastToBP_CouchCharacter OtherActor))
      (Variables|Default|SetPlayer _asbp_couch_character)))
  (Utilities|IsValid _returnvalue
    (:Is%20Valid
      (bind _asbp_interact_progress_1 (Utilities|Casting|CastToBP_InteractProgress1 _returnvalue)
        (:then
          (Default|FInit _asbp_interact_progress_1 self))
        (:CastFailed
          (Development|PrintString (Utilities|GetDisplayName _returnvalue)))))
    (:Is%20Not%20Valid
      (Development|PrintString "not valid"))))

(event EventBeginPlay
  (bind _hitmesh (Variables|Default|GetHitMesh))
  (bind _returnvalue (Transformation|GetWorldScale _hitmesh))
  ;[1 0.08664 0.08333] PlaySoundforBigHole
  (Utilities|FlowControl|Delay 0.04)
  (if (Math|Boolean|ORBoolean (> (.x _returnvalue) 0.5) (> (.y _returnvalue) 0.5) (> (.z _returnvalue) 1.0))
    (Audio|PlaySound2D "/Game/Sound/Content_Sound/Explosion_Cue.Explosion_Cue" 1.0 1.0 0.0 0 0)))

(fn ConstructionScript)