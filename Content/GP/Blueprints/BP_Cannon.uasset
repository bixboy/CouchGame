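; BP_Cannon is a cannon actor that can charge, move along one axis and offer an interaction prompt.
; Debug keys drive it: Space held starts and released stops charging, while Left and Right start and stop signed movement through functions defined outside these graphs.
; A box overlap has the widget component spawn BP_Interact at PoseWidget and destroy it on exit, without filtering the overlapping actor.
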(event OnComponentBeginOverlap(Box)
  (params (OverlappedComponent :type Primitive%20Component%20Object%20Reference) (OtherActor :type Actor%20Object%20Reference) (OtherComp :type Primitive%20Component%20Object%20Reference) (OtherBodyIndex :type Integer) (bFromSweep :type Boolean) (SweepResult :type Hit%20Result%20Structure%20%28by%20ref%29))
  (Class|CouchWidgetSpawn|SpawnWidget (Variables|Default|GetWidgetComponent) "/Game/GP/Blueprints/Widgets/3D_Widget/BP_Interact.BP_Interact_C" (Variables|Default|GetPoseWidget)))

(event OnComponentEndOverlap(Box)
  (params (OverlappedComponent :type Primitive%20Component%20Object%20Reference) (OtherActor :type Actor%20Object%20Reference) (OtherComp :type Primitive%20Component%20Object%20Reference) (OtherBodyIndex :type Integer))
  (Class|CouchWidgetSpawn|DestroyWidget (Variables|Default|GetWidgetComponent)))

(event EventBeginPlay)

(event Input|KeyboardEvents|DebugKeySpaceBar
  (params (Key :type Key%20Structure :default "None") (ActionValue :type Input%20Action%20Value%20Structure))
  (:Pressed
    (Class|CoucheCannon|StartCharging))
  (:Released
    (Class|CoucheCannon|StopCharging)))

(event Input|KeyboardEvents|DebugKeyLeft
  (params (Key :type Key%20Structure :default "None") (ActionValue :type Input%20Action%20Value%20Structure))
  (:Pressed
    (Class|CoucheCannon|StartMovement 1))
  (:Released
    (Class|CoucheCannon|StopMovement)))

(event Input|KeyboardEvents|DebugKeyRight
  (params (Key :type Key%20Structure :default "None") (ActionValue :type Input%20Action%20Value%20Structure))
  (:Pressed
    (Class|CoucheCannon|StartMovement -1))
  (:Released
    (Class|CoucheCannon|StopMovement)))

(fn ConstructionScript)