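; Fishing rod actor that casts a lure with a charge-and-release input on debug key L.
; Holding plays a timeline that scales range up to max power, tracing along the rod's forward vector and targeting the trace end.
; Releasing spawns a lure with a runtime-created cable and physics constraint to the rod, then initializes it with a suggested arc velocity toward that target.
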(event Custom|SpawnLure
  (bind _cable (CallFunction|SetCable))
  (CallFunction|SetLure _cable)
  (Game|SuggestProjectileVelocityCustomArc (Transformation|GetWorldLocation (Variables|Default|GetAttachPoint)) (Variables|Default|GetTargetLocation) 0.0 0.5))

(event Custom|Charging
  (bind _alpha (Timeline|ChargingForce PlayFromStart)
    (:Update
      (bind _output_get (Variables|Default|SetCurrentPower (* _alpha (Variables|Default|GetMaxPower))))
      (Variables|Default|SetRange _output_get)
      (bind _traceend (Utilities|GetDistance))
      (Variables|Default|SetTargetLocation _traceend))))

(event Input|KeyboardEvents|DebugKeyL
  (params (Key :type Key%20Structure :default "None") (ActionValue :type Input%20Action%20Value%20Structure))
  (:Pressed
    (CallFunction|Charging))
  (:Released
    (Audio|Components|Audio|Stop (Variables|Default|GetChargingForce))
    (CallFunction|SpawnLure)))

(fn ConstructionScript)

(fn SetCable
  (bind _returnvalue (Game|AddComponentbyClass "/Script/CableComponent.CableComponent" false))
  (Transformation|SetRelativeScale3D _returnvalue "1.000000,1.000000,1.000000")
  (Rendering|Material|SetMaterial _returnvalue 0 "/AnimationSharing/AnimSharingGreen.AnimSharingGreen")
  (Variables|/Script/CableComponent.CableComponent|SetCableLength _returnvalue 0.0)
  (return _returnvalue))

(fn SetLure
  (params (Cable :type Cable%20Component%20Object%20Reference))
  (bind _returnvalue (AddComponent|AddBPLure false))
  (Variables|Default|Setlure _returnvalue)
  (Class|CableComponent|SetAttachEndtoComponent Cable _returnvalue "")
  (Variables|/Script/CableComponent.CableComponent|SetEndLocation Cable "0, 0, 0")
  (Rendering|SetVisibility Cable true true)
  (bind _returnvalue_2 (Game|AddComponentbyClass "/Script/Engine.PhysicsConstraintComponent" false))
  (Class|PhysicsConstraintComponent|SetConstrainedComponents _returnvalue_2 (Variables|Default|GetRod) "None" (Variables|Default|Getlure) "None")
  (bind _outlaunchvelocity (Game|SuggestProjectileVelocityCustomArc (Transformation|GetActorLocation) (Variables|Default|GetTargetLocation) 0.0 0.5))
  (Class|CouchProjectile|Initialize (Variables|Default|Getlure) _outlaunchvelocity))