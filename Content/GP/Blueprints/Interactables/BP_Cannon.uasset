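; Interactable cannon Blueprint that relies on functions defined outside this graph for movement, interaction, reloading and charging.
; Overlapping its box spawns an interact-progress widget at the widget pose through the WidgetComponent, and leaving destroys it.
; Debug keys move it left or right, make player 0's couch character interact, or reload it with a newly spawned pickable cannonball.
; The charge start and stop calls are unwired.
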(event OnComponentBeginOverlap(Box)
  (params (OverlappedComponent :type Primitive%20Component%20Object%20Reference) (OtherActor :type Actor%20Object%20Reference) (OtherComp :type Primitive%20Component%20Object%20Reference) (OtherBodyIndex :type Integer) (bFromSweep :type Boolean) (SweepResult :type Hit%20Result%20Structure%20%28by%20ref%29))
  (Class|CouchWidgetSpawn|SpawnWidget (Variables|Default|GetWidgetComponent) "/Game/GP/Blueprints/Widgets/3D_Widget/BP_InteractProgress.BP_InteractProgress_C" (Variables|Default|GetWidgetPose)))

(event OnComponentEndOverlap(Box)
  (params (OverlappedComponent :type Primitive%20Component%20Object%20Reference) (OtherActor :type Actor%20Object%20Reference) (OtherComp :type Primitive%20Component%20Object%20Reference) (OtherBodyIndex :type Integer))
  (Class|CouchWidgetSpawn|DestroyWidget (Variables|Default|GetWidgetComponent)))

(event EventTick
  (params (DeltaSeconds :type Float%20%28single-precision%29)))

(event Input|KeyboardEvents|DebugKeySpaceBar
  (params (Key :type Key%20Structure :default "None") (ActionValue :type Input%20Action%20Value%20Structure)))

(event Input|KeyboardEvents|DebugKeyLeft
  (params (Key :type Key%20Structure :default "None") (ActionValue :type Input%20Action%20Value%20Structure))
  (:Pressed
    (Class|CoucheCannon|StartMovement 1))
  (:Released
    (Class|CoucheCannon|StopMovement)))

(event Input|KeyboardEvents|DebugKeyRight
  (params (Key :type Key%20Structure :default "None") (ActionValue :type Input%20Action%20Value%20Structure))
  (:Pressed
    (Class|CoucheCannon|StartMovement -1))
  (:Released
    (Class|CoucheCannon|StopMovement)))

(event Input|KeyboardEvents|DebugKey<
  (params (Key :type Key%20Structure :default "None") (ActionValue :type Input%20Action%20Value%20Structure))
  (:Pressed
    (bind _returnvalue (Game|SpawnActorfromClass "/Game/GP/Blueprints/Interactables/BP_PickableCannonBall.BP_PickableCannonBall_C" (Math|Transform|MakeTransform "0, 0, 0" "0, 0, 0" "1.000000,1.000000,1.000000") "AlwaysSpawn" "MultiplyWithRoot" 0 0))
    (Class|CoucheCannon|Reload _returnvalue)))

(event Input|KeyboardEvents|DebugKeyW
  (params (Key :type Key%20Structure :default "None") (ActionValue :type Input%20Action%20Value%20Structure))
  (:Pressed
    (bind _asbp_couch_character (Utilities|Casting|CastToBP_CouchCharacter (Game|GetPlayerCharacter 0)))
    (Class|CouchInteractable|Interact _asbp_couch_character)))

(fn ConstructionScript)