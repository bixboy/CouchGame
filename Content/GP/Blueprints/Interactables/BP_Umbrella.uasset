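; BP_Umbrella is an umbrella interactable with hit points (Pv) and a repair progress widget.
; When its interact box is overlapped, it caches the first BP_CouchCharacter as Player, then initializes the BP_RepairProgress widget with itself.
; Once Player is cached, any later overlap re-initializes the widget.
; PlayFx plays a broken sound at zero Pv, otherwise a damage sound.
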(event OnComponentBeginOverlap(BoxInteract)
  (params (OverlappedComponent :type Primitive%20Component%20Object%20Reference) (OtherActor :type Actor%20Object%20Reference) (OtherComp :type Primitive%20Component%20Object%20Reference) (OtherBodyIndex :type Integer) (bFromSweep :type Boolean) (SweepResult :type Hit%20Result%20Structure%20%28by%20ref%29))
  (bind _widgetcomponent (Variables|Default|GetWidgetComponent))
  (bind _returnvalue (Class|CouchWidgetSpawn|GetCurrentWidget _widgetcomponent))
  (Variables|Default|GetPlayer
    (:then
      _)
    (:else
      (bind _asbp_couch_character (Utilities|Casting|CastToBP_CouchCharacter OtherActor))
      (Variables|Default|SetPlayer _asbp_couch_character)))
  (Utilities|IsValid _returnvalue
    (:Is%20Valid
      (bind _asbp_repair_progress (Utilities|Casting|CastToBP_RepairProgress _returnvalue)
        (:then
          (Default|FInit _asbp_repair_progress self))
        (:CastFailed
          (Development|PrintString "Cast BP_InteractProgressBar Failed"))))))

(event EventPlayFx
  (if (== (Class|CouchUmbrella|GetCurrentPv) 0)
    (Audio|PlaySound2D (Variables|Default|GetBrokeSound) 1.0 1.0 0.0 0 0)
    (else
      (Audio|PlaySound2D (Variables|Default|GetDamageSound) 1.0 1.0 0.0 0 0))))

(fn ConstructionScript)