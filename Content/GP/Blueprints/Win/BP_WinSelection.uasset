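; BP_WinSelection stages the end-of-match win screen, showing the winning and losing teams' characters.
; Setup gathers player meshes by team from the game manager, pads each team to two and orders them by which team won.
; It applies meshes and materials to four display slots, shows eyes only for valid meshes, then snaps the main camera to its own camera's relative transform.
; A reset function restores the camera transform cached at BeginPlay.
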(event Custom|CE_ChangeSkeletalMesh
  (params (SkeletalToChange :type Skeletal%20Mesh%20Component%20Object%20Reference) (New%20Skeletal :type Skeletal%20Mesh%20Object%20Reference))
  (bind _materials (Variables|/Script/Engine.SkeletalMesh|GetMaterials New%20Skeletal))
  (Components|SkeletalMesh|SetSkeletalMeshAsset SkeletalToChange New%20Skeletal)
  (for _index (range 0 (- (Rendering|Material|GetNumMaterials SkeletalToChange) 1))
    (if (Utilities|Array|IsValidIndex _materials _index)
      (Rendering|Material|SetMaterial SkeletalToChange _index (.MaterialInterface (Utilities|Struct|BreakSkeletalMaterial (Utilities|Array|Get(acopy) _materials _index))))
      (else
        (Rendering|Material|SetMaterial SkeletalToChange _index 0)))))

(event Custom|CE_Init
  (params (Winner1 :type Skeletal%20Mesh%20Object%20Reference) (Winner2 :type Skeletal%20Mesh%20Object%20Reference) (Looser1 :type Skeletal%20Mesh%20Object%20Reference) (Looser2 :type Skeletal%20Mesh%20Object%20Reference))
  (CallFunction|FEyesVisibility Winner1 (Variables|Default|GetEyes3))
  (CallFunction|CEChangeSkeletalMesh (Variables|Default|GetWinner1) Winner1)
  (CallFunction|FEyesVisibility Winner2 (Variables|Default|GetEyes))
  (CallFunction|CEChangeSkeletalMesh (Variables|Default|GetWinner2) Winner2)
  (CallFunction|FEyesVisibility Looser1 (Variables|Default|GetEyes2))
  (CallFunction|CEChangeSkeletalMesh (Variables|Default|GetLooser1) Looser1)
  (CallFunction|FEyesVisibility Looser2 (Variables|Default|GetEyes1))
  (CallFunction|CEChangeSkeletalMesh (Variables|Default|GetLooser2) Looser2)
  (CallFunction|FMoveCamera))

(event Custom|CE_SetUpWinScreen
  (bind (_team1skins _team2skins) (CallFunction|FGetTeamSkins))
  (if (Variables|/Script/CouchGame.CouchGameManagerSubSystem|GetTeam1WinTheGame (Subsystems|GetBPGameManager))
    (CallFunction|CEInit (Utilities|Array|Get(acopy) _team1skins) (Utilities|Array|Get(acopy) _team1skins 1) (Utilities|Array|Get(acopy) _team2skins) (Utilities|Array|Get(acopy) _team2skins 1))
    (else
      (CallFunction|CEInit (Utilities|Array|Get(acopy) _team2skins) (Utilities|Array|Get(acopy) _team2skins 1) (Utilities|Array|Get(acopy) _team1skins) (Utilities|Array|Get(acopy) _team1skins 1)))))

(event EventBeginPlay
  (Variables|Default|SetStartCameraTransform (Transformation|GetActorTransform (Variables|Default|GetMainCamera))))

(event Collision|EventActorBeginOverlap
  (params (OtherActor :type Actor%20Object%20Reference)))

(event EventTick
  (params (DeltaSeconds :type Float%20%28single-precision%29)))

(fn ConstructionScript)

(fn FMoveCamera
  (Transformation|SetWorldTransform (Variables|/Script/Engine.CameraActor|GetCameraComponent (Variables|Default|GetMainCamera)) (Transformation|GetRelativeTransform (Variables|Default|GetCamera)) false true))

(fn FResetCamera
  (Transformation|SetWorldTransform (Variables|/Script/Engine.CameraActor|GetCameraComponent (Variables|Default|GetMainCamera)) (Variables|Default|GetStartCameraTransform) false true))

(fn FGetTeamSkins
  (Utilities|Array|Clear (LocalVariables|GetTeam1%20SkinsTemp))
  (Utilities|Array|Clear (LocalVariables|GetTeam2%20SkinsTemp))
  (for _array_element (Variables|/Script/CouchGame.CouchGameManagerSubSystem|GetPlayers (Subsystems|GetBPGameManager))
    (if (== (.teamindex _array_element) 1)
      (Utilities|Array|Add (LocalVariables|GetTeam1%20SkinsTemp) (.skeletalmeshasset _array_element))
      (else
        (Utilities|Array|Add (LocalVariables|GetTeam2%20SkinsTemp) (.skeletalmeshasset _array_element)))))
  (while (< (Utilities|Array|Length (LocalVariables|GetTeam1%20SkinsTemp)) 2)
    (Utilities|Array|Add (LocalVariables|GetTeam1%20SkinsTemp) 0))
  (while (< (Utilities|Array|Length (LocalVariables|GetTeam2%20SkinsTemp)) 2)
    (Utilities|Array|Add (LocalVariables|GetTeam2%20SkinsTemp) 0))
  (return (LocalVariables|GetTeam1%20SkinsTemp) (LocalVariables|GetTeam2%20SkinsTemp)))

(fn FEyesVisibility
  (params (Skeletal :type Skeletal%20Mesh%20Object%20Reference) (Eyes :type Static%20Mesh%20Component%20Object%20Reference))
  (Utilities|IsValid Skeletal
    (:Is%20Valid
      (Rendering|SetVisibility Eyes true false))
    (:Is%20Not%20Valid
      (Rendering|SetVisibility Eyes false false)))
  (return))